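; BP_Computer is an interactable computer actor that opens a ComputerWidget UI on screen.
; On BeginPlay it enables input for player controller 0 on authority, and its Trigger overlap events toggle an IsOverlapped flag without filtering actors.
; Pressing F while overlapped clears all widgets and adds a new ComputerWidget to the viewport.
; Q leads to a widget-removal branch with a constant false condition, so it closes nothing.
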(event `self.ReceiveBeginPlay`
  (`/Engine/EditorBlueprintResources/ActorMacros.Switch Has Authority`
    (:`Authority`
      (`self.EnableInput` (`GameplayStatics.GetPlayerController` 0)))))

(event `Key|F`
  (params (Key :type "Key Structure"))
  (:`Pressed`
    (if (`self.IsOverlapped`)
      (`WidgetLayoutLibrary.RemoveAllWidgets`)
      (bind _returnvalue (`|CreateWidget` "/Game/UI/ComputerWidget.ComputerWidget_C"))
      (bind _output_get (set `self.NewVar` _returnvalue))
      (`UserWidget.AddToViewport` _output_get 0)
      (if false :!label _label
        (`WidgetLayoutLibrary.RemoveAllWidgets`)))))

(event `Key|Q`
  (params (Key :type "Key Structure"))
  (:`Pressed`
    (goto _label)))

(event `self.Trigger.OnComponentBeginOverlap`
  (params (OverlappedComponent :type "PrimitiveComponent Object Reference") (OtherActor :type "Actor Object Reference") (OtherComp :type "PrimitiveComponent Object Reference") (OtherBodyIndex :type Integer) (bFromSweep :type Boolean) (SweepResult :type "HitResult Structure (by ref)"))
  (set `self.IsOverlapped` true))

(event `self.Trigger.OnComponentEndOverlap`
  (params (OverlappedComponent :type "PrimitiveComponent Object Reference") (OtherActor :type "Actor Object Reference") (OtherComp :type "PrimitiveComponent Object Reference") (OtherBodyIndex :type Integer))
  (set `self.IsOverlapped` false))

(fn `UserConstructionScript`)